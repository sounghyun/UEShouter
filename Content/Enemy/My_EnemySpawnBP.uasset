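; Enemy spawner actor that keeps adding My_EnemyBP AI pawns to the level up to a fixed population cap.
; On BeginPlay it caches My_GamoMode and starts a looping half-second timer that calls EnemySpawn.
; While the game mode's EnemyNum is below ten, each tick of that timer increments the count and spawns an enemy at a random point inside the SpawnPoints box.
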(event Custom|EnemySpawn
  (bind _spawnpoints (Variables|Default|GetSpawnPoints))
  (bind _gamemode (Variables|Default|GetGameMode))
  (if (< (Variables|/Game/My_GamoMode.My_GamoMode_C|GetEnemyNum _gamemode) 1e+01)
    (Default|EnemyNumUP _gamemode)
    (AI|SpawnAIFromClass "/Game/Enemy/My_EnemyBP.My_EnemyBP_C" 0 (Math|Random|RandomPointinBoundingBox (Transformation|GetWorldLocation _spawnpoints) (Variables|/Script/Engine.BoxComponent|GetBoxExtent _spawnpoints)) "0, 0, 0" false)))

(event EventBeginPlay
  (bind _asmy_gamo_mode (Utilities|Casting|CastToMy_GamoMode (Game|GetGameMode)))
  (Variables|Default|SetGameMode _asmy_gamo_mode)
  (Utilities|Time|SetTimerbyFunctionName 0 "EnemySpawn" 0.5 true))

(event Collision|EventActorBeginOverlap
  (params (OtherActor :type Actor%20Object%20Reference)))

(event EventTick
  (params (DeltaSeconds :type Float%20%28single-precision%29)))

(fn ConstructionScript)