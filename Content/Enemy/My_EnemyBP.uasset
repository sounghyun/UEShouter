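; My_EnemyBP is an enemy actor that holds HP and damages the hero while overlapping it.
; An overlapping damageable hero starts a looping timer that calls Attack to deal damage through DownHPMessage.
; Any overlap ending clears that timer.
; DownHP lowers HP and, at zero, tells the cached game mode to decrement the enemy count before destroying the actor.
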(event Custom|Attack
  (Class|MyDamegeInterFaceBP|DownHP(Message) (Variables|Default|GetHero) 1e+01))

(event EventBeginPlay
  (bind _asmy_gamo_mode (Utilities|Casting|CastToMy_GamoMode (Game|GetGameMode)))
  (Variables|Default|SetGameMode _asmy_gamo_mode)
  (Variables|Default|SetHP 1e+02))

(event Collision|EventActorBeginOverlap
  (params (OtherActor :type Actor%20Object%20Reference))
  (if (Utilities|DoesObjectImplementInterface OtherActor "/Game/Interface/My_DamegeInterFaceBP.My_DamegeInterFaceBP_C")
    (bind _asmy_hero_bp (Utilities|Casting|CastToMy_HeroBP OtherActor))
    (Variables|Default|SetHero _asmy_hero_bp)
    (Utilities|Time|SetTimerbyFunctionName 0 "Attack" 0.33 true)))

(event EventDownHP
  (params (DisHP :type Float%20%28single-precision%29))
  (bind _output_get (Variables|Default|SetHP (- (Variables|Default|GetHP) DisHP)))
  (if (<= _output_get 0.0)
    (Default|EnemyNumDown (Variables|Default|GetGameMode))
    (Actor|DestroyActor)))

(event EventTick
  (params (DeltaSeconds :type Float%20%28single-precision%29)))

(event Collision|EventActorEndOverlap
  (params (OtherActor :type Actor%20Object%20Reference))
  (Utilities|Time|ClearTimerbyFunctionName 0 "Attack"))

(fn ConstructionScript)